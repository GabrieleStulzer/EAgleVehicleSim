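; BP_Track is a construction-script actor that lines a spline track with blue cones on one side and yellow cones on the other.
; Cone spacing comes from the cone mesh's X bounds plus Offset, and spline length sets the instance count.
; At each step it rotates the normalized tangent ±90 degrees for a fixed sideways offset, adding tangent-aligned mesh instances in local space.
; The event graph has no active logic.
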(fn `UserConstructionScript`
  (bind (_min _max) (break `Box` (`StaticMesh.GetBoundingBox` (`self.ConeMesh`))))
  (`StaticMeshComponent.SetStaticMesh` (`self.BlueCones`) (`self.ConeMesh`))
  (`StaticMeshComponent.SetStaticMesh` (`self.YellowCones`) (`self.OrangeConeMesh`))
  (bind _output_get (set `self.Spacing` (+ (.x (- _max _min)) (`self.Offset`))))
  (bind _output_get_2 (set `self.NumberOfInstances` (`KismetMathLibrary.FFloor` (/ (`SplineComponent.GetSplineLength` (`self.Track`)) _output_get))))
  (for _index (range (+ _output_get_2 1))
    (`/Engine/EditorBlueprintResources/StandardMacros.NegateFloat` (`self.LateralOffset`)
      (:`  `
        (bind _returnvalue (* _index (`self.Spacing`)))
        (bind _returnvalue_2 (`SplineComponent.GetLocationAtDistanceAlongSpline` (`self.Track`) _returnvalue "Local"))
        (bind _returnvalue_3 (`SplineComponent.GetTangentAtDistanceAlongSpline` (`self.Track`) _returnvalue "Local"))
        (bind _returnvalue_4 (`KismetMathLibrary.Normal` _returnvalue_3))
        (bind _returnvalue_5 (`KismetMathLibrary.MakeRotFromX` _returnvalue_3))
        (`InstancedStaticMeshComponent.AddInstance` (`self.BlueCones`) (`KismetMathLibrary.MakeTransform` (+ _returnvalue_2 (* (`KismetMathLibrary.GreaterGreater_VectorRotator` _returnvalue_4 (struct :`Yaw` 90.0)) 100)) _returnvalue_5) false)
        (`InstancedStaticMeshComponent.AddInstance` (`self.YellowCones`) (`KismetMathLibrary.MakeTransform` (+ _returnvalue_2 (* (`KismetMathLibrary.GreaterGreater_VectorRotator` _returnvalue_4 (struct :`Yaw` -90.0)) 100)) _returnvalue_5) false)))))